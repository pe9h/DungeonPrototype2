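; Simple chasing AI pawn in the wave-based spawner content that pursues a randomly chosen player's pawn.
; On BeginPlay, only the authority picks the target from the GameState PlayerArray via the owning PlayerController.
; It then reissues AIMoveTo on a short delay loop without waiting for move results.
; The target is chosen once and never reselected.
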(event EventBeginPlay
  (Networking|SwitchHasAuthority
    (:Authority
      ;[1 1 1] Select a target
      (Variables|Default|SettargetPawn (Pawn|GetControlledPawn (.AsPlayer%20Controller (Utilities|Casting|CastToPlayerController (Components|GetOwner (.OutItem (Utilities|Array|Random (Variables|/Script/Engine.GameStateBase|GetPlayerArray (Game|GetGameState)))))))))
      ;[1 1 1] Chase until the end of the earth
      (AI|AIMoveTo self "0, 0, 0" (Variables|Default|GettargetPawn) 5.0 false :!label _label
        (:then
          (Utilities|FlowControl|Delay 0.2)
          (goto _label))))))

(fn ConstructionScript)